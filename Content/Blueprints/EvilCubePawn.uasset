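; EvilCubePawn is a destructible target pawn that awards score to the first-person game mode.
; Any hit on its cube component spawns an explosion effect at the cube's transform and destroys that component.
; When the explosion's end-play event fires, the pawn destroys itself and passes its score value to FirstPersonGameMode, so points arrive after the effect finishes.
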(event `self.Cube.OnComponentHit`
  (params (HitComponent :type "PrimitiveComponent Object Reference") (OtherActor :type "Actor Object Reference") (OtherComp :type "PrimitiveComponent Object Reference") (NormalImpulse :type "Vector Structure") (Hit :type "HitResult Structure (by ref)"))
  (`|ExecutionSequence`
    (:`then_0`
      (bind _returnvalue (`|SpawnActorFromClass` "/Game/StarterContent/Blueprints/Blueprint_Effect_Explosion.Blueprint_Effect_Explosion_C" (`SceneComponent.K2_GetComponentToWorld` (`self.Cube`)) "Undefined" "OverrideRootScale" null null))
      (set `self.varExposion` _returnvalue))
    (:`then_1`
      (`ActorComponent.K2_DestroyComponent` (`self.Cube`)))))

(event `self.varExposion.OnEndPlay`
  (params (Actor :type "Actor Object Reference") (EndPlayReason :type "EEndPlayReason Enum" :default "Destroyed"))
  (`self.K2_DestroyActor`)
  (bind _asfirst_person_game_mode (cast `/Game/FirstPersonBP/Blueprints/FirstPersonGameMode` (`GameplayStatics.GetGameMode`)))
  (`/Game/FirstPersonBP/Blueprints/FirstPersonGameMode.CE_AddTargetScore` _asfirst_person_game_mode (`self.varScoreValue`)))

(fn `UserConstructionScript`)